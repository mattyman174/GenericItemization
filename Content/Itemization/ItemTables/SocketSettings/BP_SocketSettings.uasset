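; Socket settings Blueprint for the itemization system that decides which socket definitions are active on an item instance.
; DetermineActiveSockets gives a valid instance a one-in-three chance to roll sockets, then picks a random count capped by quality type.
; Normal items can roll up to every defined socket, Magic items up to half, and other qualities none.
; Active sockets are always the first indices in definition order, and a roll can yield zero.
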(fn DetermineActiveSockets
  (params (ItemInstance :type Instanced%20Struct%20Structure%20%28by%20ref%29) (ItemInstancingContext :type Instanced%20Struct%20Structure%20%28by%20ref%29))
  (bind _socketdefinitions (Variables|Default|GetSocketDefinitions))
  (bind _returnvalue (Utilities|Array|Length _socketdefinitions))
  (bind _value (Class|StructUtilsFunctionLibrary|GetInstancedStructValue ItemInstance)
    (:Valid
      (if (== (Math|Random|RandomIntegerinRange 1 3) 1) ; Sockets have a 1 in 3 chance of spawning at all.
        (for _index (range 0 (- (Math|Random|RandomIntegerinRange 0 (select (== (Utilities|Struct|BreakItemInstance _value) "(TagName=\"Itemization.QualityType.Normal\")") _returnvalue (select (== (Utilities|Struct|BreakItemInstance _value) "(TagName=\"Itemization.QualityType.Magic\")") (/ _returnvalue 2) 0))) 1)) ; Normal and Magic Items can spawn a number of Sockets.
          (Utilities|Array|Add (LocalVariables|GetLocalSocketIndexes) _index))
        (return (LocalVariables|GetLocalSocketIndexes) true)
        (else
          _)))
    (:NotValid
      _))
  (return (LocalVariables|GetLocalSocketIndexes) true))