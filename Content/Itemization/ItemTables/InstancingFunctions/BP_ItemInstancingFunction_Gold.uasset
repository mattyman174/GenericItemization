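; Item instancing function that decides the stack count of Gold items when they are instanced.
; Overrides CalculateStackCount, unwrapping the item and context structs to confirm the Gold item type, then multiplies item level by a small random roll.
; A positive Gold Multiplier mutator scales the result after truncation and integer division by 256.
; Non-Gold items or invalid structs fall back to the parent implementation.
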(fn CalculateStackCount
  (params (ItemInstance :type Instanced%20Struct%20Structure%20%28by%20ref%29) (ItemInstancingContext :type Instanced%20Struct%20Structure%20%28by%20ref%29))
  (bind _value (Class|StructUtilsFunctionLibrary|GetInstancedStructValue ItemInstance)
    (:Valid
      (bind _value_2 (Class|StructUtilsFunctionLibrary|GetInstancedStructValue (Utilities|Struct|BreakItemInstance _value))
        (:Valid
          (if (== (Utilities|Struct|BreakItemDefinition _value_2) "(TagName=\"Itemization.ItemType.Gold\")") ; Verify we are actually calculating StackCount for Gold.
            (bind _value_3 (Class|StructUtilsFunctionLibrary|GetInstancedStructValue ItemInstancingContext)
              (:Valid
                (return (* (* (.ItemLevel (Utilities|Struct|BreakItemInstancingContext _value_3)) (Math|Random|RandomIntegerinRange 1 6)) (select (and (.ReturnValue (Utilities|Map|Find (.Mutators (Utilities|Struct|BreakItemInstancingContext _value_3)) "(TagName=\"Itemization.Mutator.Gold.Multiplier\")")) (> (Math|Float|Truncate (.value (.Value (Utilities|Map|Find (.Mutators (Utilities|Struct|BreakItemInstancingContext _value_3)) "(TagName=\"Itemization.Mutator.Gold.Multiplier\")")))) 0)) (/ (Math|Float|Truncate (.value (.Value (Utilities|Map|Find (.Mutators (Utilities|Struct|BreakItemInstancingContext _value_3)) "(TagName=\"Itemization.Mutator.Gold.Multiplier\")")))) 256) 1)) true))
              (:NotValid
                _))))
        (:NotValid
          _)))
    (:NotValid
      _))
  (bind (_outstackcount _returnvalue) (|CallParentFunction ItemInstance ItemInstancingContext))
  (return _outstackcount _returnvalue))