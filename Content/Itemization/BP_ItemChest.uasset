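; Item chest that opens when something overlaps its interaction sphere and closes when the overlap ends.
; A timeline swings the lid, while a burst effect and sound play after a short delay.
; After that delay, the server destroys previous drops and requests new ones from the ItemDropperComponent.
; Each drop teleports to a random reachable point within the sphere's radius, retrying any point too close to the chest.
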(event OnComponentBeginOverlap(InteractionVolume)
  (params (OverlappedComponent :type Primitive%20Component%20Object%20Reference) (OtherActor :type Actor%20Object%20Reference) (OtherComp :type Primitive%20Component%20Object%20Reference) (OtherBodyIndex :type Integer) (bFromSweep :type Boolean) (SweepResult :type Hit%20Result%20Structure%20%28by%20ref%29))
  (CallFunction|OpenChest))

(event OnComponentEndOverlap(InteractionVolume)
  (params (OverlappedComponent :type Primitive%20Component%20Object%20Reference) (OtherActor :type Actor%20Object%20Reference) (OtherComp :type Primitive%20Component%20Object%20Reference) (OtherBodyIndex :type Integer))
  (CallFunction|CloseChest))

(event Custom|OpenChest
  (bind _chestlid (Variables|Default|GetChestLid))
  (bind _returnvalue (Transformation|GetWorldLocation _chestlid))
  (Utilities|FlowControl|Sequence
    (:then_0
      (Utilities|FlowControl|Delay 0.5)
      (Niagara|SpawnSystematLocation "/Niagara/DefaultAssets/Templates/Systems/RadialBurst.RadialBurst" _returnvalue)
      (Audio|SpawnSoundatLocation "/Game/Assets/Sounds/UI/A_UI_Select02.A_UI_Select02" _returnvalue "0, 0, 0" 1.0 1.0 0.0 0 0)
      ;[1 0 0] When the Chest Opens on the Server, get it to Drop some Items and randomly scatter them around.
      (Networking|SwitchHasAuthority
        (:Authority
          (for _array_element (Variables|Default|GetItem%20Drops)
            (Utilities|IsValid _array_element
              (:Is%20Valid
                (Actor|DestroyActor _array_element))))
          (bind _returnvalue_2 (Class|StructUtilsFunctionLibrary|MakeInstancedStruct (Variables|GenericItemization|GetUserContextData)))
          (bind (_itemdrops _returnvalue_3) (Class|ItemDropperComponent|DropItems (Variables|Default|GetItemDropperComponent) _returnvalue_2))
          (if _returnvalue_3
            (bind _output_get (Variables|Default|SetItem%20Drops _itemdrops))
            (for _array_element_2 _output_get
              (bind _output_get_2 (Variables|Default|SetNewLocation (.RandomLocation (AI|Navigation|GetRandomReachablePointinRadius (Transformation|GetActorLocation) (Class|SphereComponent|GetUnscaledSphereRadius (Variables|Default|GetInteractionVolume)) 0 0)) :!label _label))
              (if (> (Math|Vector|Distance(Vector) _output_get_2 (Transformation|GetActorLocation)) 5e+01)
                (Transformation|SetActorLocation _array_element_2 _output_get_2 false true)
                (else
                  (goto _label))))
            (else
              (Development|PrintString "Dropped No Items!" true true "(R=1.000000,G=0.000000,B=0.000000,A=1.000000)")
              (Utilities|Array|Clear (Variables|Default|GetItem%20Drops)))))))
    (:then_1
      (bind _lidroll (Timeline|OpenLid PlayFromStart)
        (:Update
          (Transformation|SetRelativeRotation (Variables|Default|GetLidPivot) (Math|Rotator|MakeRotator _lidroll 0.0 0.0) false false))))))

(event Custom|CloseChest
  (Utilities|FlowControl|Sequence
    (:then_0
      (bind _lidroll (Timeline|OpenLid Reverse)
        (:Update
          (Transformation|SetRelativeRotation (Variables|Default|GetLidPivot) (Math|Rotator|MakeRotator _lidroll 0.0 0.0) false false))))))

(fn ConstructionScript)