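; Character inventory component Blueprint that plays a pickup sound for gold.
; It handles both the item-added and stack-count-changed events, unwrapping the item's instanced struct and then its item definition to read the item type.
; If the type is Gold, it plays the ItemPickup sound in 2D.
; The stack event does not check direction, so any change in a gold stack's count triggers the sound.
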(event EventOnAddedItem
  (params (Item :type Instanced%20Struct%20Structure%20%28by%20ref%29) (UserContextData :type Instanced%20Struct%20Structure%20%28by%20ref%29))
  (bind _value (Class|StructUtilsFunctionLibrary|GetInstancedStructValue Item)
    (:Valid
      (bind _value_2 (Class|StructUtilsFunctionLibrary|GetInstancedStructValue (Utilities|Struct|BreakItemInstance _value))
        (:Valid
          (if (== (Utilities|Struct|BreakItemDefinition _value_2) "(TagName=\"Itemization.ItemType.Gold\")")
            (Audio|PlaySound2D "/Game/Itemization/Inventories/ItemPickup.ItemPickup" 1.0 1.0 0.0 0 0)))))))

(event EventOnItemStackCountChanged
  (params (Item :type Instanced%20Struct%20Structure%20%28by%20ref%29) (UserContextData :type Instanced%20Struct%20Structure%20%28by%20ref%29) (OldStackCount :type Integer) (NewStackCount :type Integer))
  (bind _value (Class|StructUtilsFunctionLibrary|GetInstancedStructValue Item)
    (:Valid
      (bind _value_2 (Class|StructUtilsFunctionLibrary|GetInstancedStructValue (Utilities|Struct|BreakItemInstance _value))
        (:Valid
          (if (== (Utilities|Struct|BreakItemDefinition _value_2) "(TagName=\"Itemization.ItemType.Gold\")")
            (Audio|PlaySound2D "/Game/Itemization/Inventories/ItemPickup.ItemPickup" 1.0 1.0 0.0 0 0)))))))