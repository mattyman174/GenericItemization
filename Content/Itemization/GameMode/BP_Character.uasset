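; BP_Character is the itemization game mode's character Blueprint, which puts the inventory widget on screen for the local player.
; On Restarted, a locally controlled character re-adds its cached inventory widget to the viewport if one is valid.
; Otherwise it creates WBP_CharacterInventory, owned by its BP_PlayerController and bound to that controller's inventory component, then caches and displays it.
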(event EventRestarted
  (|CallParentFunction)
  (if (Pawn|IsLocallyControlled)
    (Utilities|IsValid (Variables|Default|GetInventoryWidget)
      (:Is%20Valid
        (UserInterface|Viewport|AddtoViewport (Variables|Default|GetInventoryWidget) 0))
      (:Is%20Not%20Valid
        (bind _asbp_player_controller (Utilities|Casting|CastToBP_PlayerController (Pawn|GetController)))
        (bind _returnvalue (UserInterface|CreateWidget "/Game/Itemization/Inventories/WBP_CharacterInventory.WBP_CharacterInventory_C" _asbp_player_controller (Variables|/Game/Itemization/GameMode/BP_PlayerController.BP_PlayerController_C|GetBP_CharacterInventoryComponent _asbp_player_controller)))
        (bind _output_get (Variables|Default|SetInventoryWidget _returnvalue))
        (UserInterface|Viewport|AddtoViewport _output_get 0)))))

(fn ConstructionScript
  (|CallParentFunction))