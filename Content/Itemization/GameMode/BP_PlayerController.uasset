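; Player controller for an itemization game mode, handling item pickup, dropping and moving items between a cursor inventory and the character inventory.
; Picked-up items go to the cursor inventory, while gold goes straight into the character inventory, stacking when possible; destination clicks drop a held cursor item.
; Guarded requests run on the server, which sockets, stacks, swaps or places items, scatters drops near the pawn, and reports pickup and drop results to the client.
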(event Custom|ServerTryPickupItem
  (params (ItemDrop :type Item%20Drop%20Object%20Reference))
  (CallFunction|ServerTryPickupItemImplementation ItemDrop))

(event Custom|TryPickupItem
  (params (ItemDrop :type Item%20Drop%20Object%20Reference))
  (if (not (Variables|Default|GetbPickingUpItem))
    (Variables|Default|SetbPickingUpItem (not (== (.ItemType (Utilities|Struct|BreakItemDefinition (Class|ItemDrop|GetItemDefinitionStruct ItemDrop))) "(TagName=\"Itemization.ItemType.Gold\")"))) ; We immediately grab Gold instead of picking it up.
    (CallFunction|ServerTryPickupItem ItemDrop)))

(event Custom|TrySwapInventoryItems
  (params (CursorInventoryItem :type Guid%20Structure) (CharacterInventoryItem :type Guid%20Structure) (CharacterInventorySlotId :type Integer))
  (bind _bsuccessful (Class|ItemInventoryComponent|GetItem (Variables|Default|GetBP_CursorInventoryComponent) CursorInventoryItem))
  (bind _bsuccessful_2 (Class|ItemInventoryComponent|GetItem (Variables|Default|GetBP_CharacterInventoryComponent) CharacterInventoryItem))
  (if (or _bsuccessful_2 _bsuccessful)
    (CallFunction|ServerTrySwapInventoryItems CursorInventoryItem CharacterInventoryItem CharacterInventorySlotId)))

(event Custom|ServerTryDropGold
  (CallFunction|ServerTryDropGoldImplementation))

(event Custom|ClientSucceededItemDrop
  (params (ItemToDrop :type Guid%20Structure))
  (Variables|Default|SetbDroppingItem false)
  (Variables|Default|SetbShowMouseCursor true))

(event Custom|ClientSucceededItemPickup
  (params (PickupItemInstance :type Instanced%20Struct%20Structure))
  (Variables|Default|SetbPickingUpItem false)
  (bind _value (Class|StructUtilsFunctionLibrary|GetInstancedStructValue PickupItemInstance)
    (:Valid
      (bind _value_2 (Class|StructUtilsFunctionLibrary|GetInstancedStructValue (Utilities|Struct|BreakItemInstance _value))
        (:Valid
          (Variables|Default|SetbShowMouseCursor (== (Utilities|Struct|BreakItemDefinition _value_2) "(TagName=\"Itemization.ItemType.Gold\")")))
        (:NotValid
          (Variables|Default|SetbShowMouseCursor false :!label _label))))
    (:NotValid
      (goto _label))))

(event Custom|ServerTryDropCursorItem
  (params (ItemToDrop :type Guid%20Structure))
  (bind (_outitemdrop _returnvalue) (Class|ItemInventoryComponent|DropItem (Variables|Default|GetBP_CursorInventoryComponent) ItemToDrop))
  (if (not _returnvalue)
    (CallFunction|ClientFailedItemDrop ItemToDrop)
    (else
      (CallFunction|SetItemDropLocation _outitemdrop)
      (CallFunction|ClientSucceededItemDrop ItemToDrop))))

(event Custom|ClientFailedItemDrop
  (params (ItemToDrop :type Guid%20Structure))
  (Variables|Default|SetbDroppingItem false)
  (Development|PrintString "FAILED TO DROP ITEM" true true "(R=1.000000,G=0.000000,B=0.000000,A=1.000000)"))

(event Custom|TryDropCursorItem
  (if (not (Variables|Default|GetbDroppingItem))
    (bind _returnvalue (Class|ItemInventoryComponent|GetItems (Variables|Default|GetBP_CursorInventoryComponent)))
    (bind _value (Class|StructUtilsFunctionLibrary|GetInstancedStructValue (Utilities|Array|Get(acopy) _returnvalue))
      (:Valid
        (Variables|Default|SetbDroppingItem true)
        (CallFunction|ServerTryDropCursorItem (Utilities|Struct|BreakItemInstance _value))))))

(event Custom|ServerTrySwapInventoryItems
  (params (CursorInventoryItem :type Guid%20Structure) (CharacterInventoryItem :type Guid%20Structure) (CharacterInventorySlotId :type Integer))
  (bind _bp_characterinventorycomponent (Variables|Default|GetBP_CharacterInventoryComponent))
  (bind (_bsuccessful _returnvalue) (Class|ItemInventoryComponent|GetItem (Variables|Default|GetBP_CursorInventoryComponent) CursorInventoryItem))
  (bind _bsuccessful_2 (Class|ItemInventoryComponent|GetItem (Variables|Default|GetBP_CharacterInventoryComponent) CharacterInventoryItem))
  (if (and _bsuccessful_2 _bsuccessful)
    (bind (_outsocketid _returnvalue_2) (Class|ItemInventoryComponent|CanSocketItem _bp_characterinventorycomponent _returnvalue CharacterInventoryItem))
    (if _returnvalue_2
      (bind _outitem (Class|ItemInventoryComponent|ReleaseItem (Variables|Default|GetBP_CursorInventoryComponent) CursorInventoryItem))
      (Class|ItemInventoryComponent|SocketItem _bp_characterinventorycomponent _outitem CharacterInventoryItem _outsocketid)
      (else
        (CallFunction|SwapItems CursorInventoryItem CharacterInventoryItem CharacterInventorySlotId :!label _label)))
    (else
      (goto _label))))

(event Custom|ClientFailedItemPickup
  (params (ItemDrop :type Item%20Drop%20Object%20Reference))
  (Variables|Default|SetbPickingUpItem false)
  (Variables|Default|SetbShowMouseCursor true)
  (Development|PrintString "FAILED TO PICKUP ITEM" true true "(R=1.000000,G=0.000000,B=0.000000,A=1.000000)"))

(event Custom|TryDropGold
  (if (not (Variables|Default|GetbDroppingItem))
    (bind _returnvalue (CallFunction|HasGold))
    (if _returnvalue
      (Variables|Default|SetbDroppingItem true)
      (CallFunction|ServerTryDropGold))))

(event EventOnSetDestinationReleased
  (if (== (Class|ItemInventoryComponent|GetNumItems (Variables|Default|GetBP_CursorInventoryComponent)) 1)
    (CallFunction|TryDropCursorItem)
    (else
      (|CallParentFunction))))

(event EventOnSetDestinationTriggered
  (if (== (Class|ItemInventoryComponent|GetNumItems (Variables|Default|GetBP_CursorInventoryComponent)) 1)
    (CallFunction|TryDropCursorItem)
    (else
      (|CallParentFunction))))

(event EventBeginPlay
  (|CallParentFunction)
  (if (Pawn|IsLocalPlayerController)
    (CallFunction|CreateCursorInventoryWidget)))

(fn ConstructionScript)

(fn CreateCursorInventoryWidget
  (bind _returnvalue (UserInterface|CreateWidget "/Game/Itemization/Inventories/WBP_CursorInventory.WBP_CursorInventory_C" self (Variables|Default|GetBP_CursorInventoryComponent)))
  (bind _output_get (Variables|Default|SetCursorInventoryWidget _returnvalue))
  (UserInterface|Viewport|AddtoViewport _output_get 1))

(fn SetItemDropLocation
  (params (ItemDrop :type Item%20Drop%20Object%20Reference))
  (bind _returnvalue (Pawn|GetControlledPawn))
  (Utilities|IsValid ItemDrop
    (:Is%20Valid
      (Utilities|IsValid _returnvalue
        (:Is%20Valid
          (bind _output_get (LocalVariables|SetLocalHitLocation (Transformation|GetActorLocation _returnvalue)))
          (bind _output_get_2 (LocalVariables|SetLocalNewLocation (.RandomLocation (AI|Navigation|GetRandomReachablePointinRadius _output_get 5e+01 0 0)) :!label _label))
          (if (> (Math|Vector|Distance(Vector) _output_get_2 _output_get) 5e+01)
            (Transformation|SetActorLocation ItemDrop _output_get_2 false true)
            (else
              (goto _label))))))))

(fn SwapItems
  (params (CursorInventoryItem :type Guid%20Structure) (CharacterInventoryItem :type Guid%20Structure) (CharacterInventorySlotId :type Integer))
  (Networking|SwitchHasAuthority
    (:Authority
      (Utilities|FlowControl|Sequence
        (:then_0
          (bind (_bsuccessful _returnvalue) (Class|ItemInventoryComponent|GetItem (Variables|Default|GetBP_CursorInventoryComponent) CursorInventoryItem))
          (bind _output_get (LocalVariables|SetbLocalHasCursorItem _bsuccessful))
          (if _output_get
            (LocalVariables|SetLocalCursorItem _returnvalue)
            (bind _returnvalue_2 (Class|ItemInventoryComponent|GetItemContextData (Variables|Default|GetBP_CursorInventoryComponent) CursorInventoryItem))
            (LocalVariables|SetLocalCursorItemContextData _returnvalue_2)))
        (:then_1
          (bind (_bsuccessful_2 _returnvalue_3) (Class|ItemInventoryComponent|GetItem (Variables|Default|GetBP_CharacterInventoryComponent) CharacterInventoryItem))
          (bind _output_get_2 (LocalVariables|SetbLocalHasCharacterItem _bsuccessful_2))
          (if _output_get_2
            (LocalVariables|SetLocalCharacterItem _returnvalue_3)
            (bind _returnvalue_4 (Class|ItemInventoryComponent|GetItemContextData (Variables|Default|GetBP_CharacterInventoryComponent) CharacterInventoryItem))
            (LocalVariables|SetLocalCharacterItemContextData _returnvalue_4)))
        (:then_2
          (if (and (LocalVariables|GetbLocalHasCursorItem) (LocalVariables|GetbLocalHasCharacterItem)) ; We might be able to perform a Swap.
            (bind _value (Class|StructUtilsFunctionLibrary|GetInstancedStructValue (LocalVariables|GetLocalCursorItem))
              (:Valid
                (bind _value_2 (Class|StructUtilsFunctionLibrary|GetInstancedStructValue (LocalVariables|GetLocalCharacterItem))
                  (:Valid
                    (bind _returnvalue_5 (Class|ItemInventoryComponent|CanStackItems (Variables|Default|GetBP_CharacterInventoryComponent) (Variables|Default|GetBP_CursorInventoryComponent) (.ItemId (Utilities|Struct|BreakItemInstance _value)) (.ItemId (Utilities|Struct|BreakItemInstance _value_2))))
                    (if _returnvalue_5 ; If we can Stack them, we should do that instead of Swapping.
                      (bind _returnvalue_6 (Class|ItemInventoryComponent|StackItemfromInventory (Variables|Default|GetBP_CharacterInventoryComponent) (Variables|Default|GetBP_CursorInventoryComponent) (.ItemId (Utilities|Struct|BreakItemInstance _value)) (.ItemId (Utilities|Struct|BreakItemInstance _value_2))))
                      (return _returnvalue_6)
                      (else
                        ;[1 0 0] Release both Items from their respective Inventories, then Swap them by Taking them for the Inventory they need to be placed in.
                        (bind _outitem (Class|ItemInventoryComponent|ReleaseItem (Variables|Default|GetBP_CursorInventoryComponent) CursorInventoryItem))
                        (bind _outitem_2 (Class|ItemInventoryComponent|ReleaseItem (Variables|Default|GetBP_CharacterInventoryComponent) CharacterInventoryItem))
                        (Class|ItemInventoryComponent|TakeItem (Variables|Default|GetBP_CursorInventoryComponent) _outitem_2)
                        (bind _returnvalue_7 (Class|StructUtilsFunctionLibrary|MakeInstancedStruct (Utilities|Struct|MakeBP_InventorySlotUserContextData CharacterInventorySlotId)))
                        (Class|ItemInventoryComponent|TakeItem (Variables|Default|GetBP_CharacterInventoryComponent) _outitem _returnvalue_7)
                        (return true))))
                  (:NotValid
                    _)))
              (:NotValid
                _))
            (return false)
            (elif (and (LocalVariables|GetbLocalHasCharacterItem) (not (LocalVariables|GetbLocalHasCursorItem))) ; No Cursor Item, pickup Character Inventory Item
              ;[1 0 0] Release just the Character Inventory Item, then place it into the Cursor Inventory.
              (bind _outitem_3 (Class|ItemInventoryComponent|ReleaseItem (Variables|Default|GetBP_CharacterInventoryComponent) CharacterInventoryItem))
              (Class|ItemInventoryComponent|TakeItem (Variables|Default|GetBP_CursorInventoryComponent) _outitem_3)
              (return true)
              (elif (and (LocalVariables|GetbLocalHasCursorItem) (not (LocalVariables|GetbLocalHasCharacterItem))) ; No Character Inventory Item, place Cursor Item
                ;[1 0 0] Release just the Cursor Inventory Item, then place it into the Character Inventory, providing the SlotId via the ContextData.
                (bind _outitem_4 (Class|ItemInventoryComponent|ReleaseItem (Variables|Default|GetBP_CursorInventoryComponent) CursorInventoryItem))
                (bind _returnvalue_8 (Class|StructUtilsFunctionLibrary|MakeInstancedStruct (Utilities|Struct|MakeBP_InventorySlotUserContextData CharacterInventorySlotId)))
                (Class|ItemInventoryComponent|TakeItem (Variables|Default|GetBP_CharacterInventoryComponent) _outitem_4 _returnvalue_8)
                (return true)
                (else
                  (return false) ; Error?
                )))))))
    (:Remote
      (return false))))

(fn ServerTryDropGoldImplementation
  (bind _returnvalue (Class|ItemInventoryComponent|GetItems (Variables|Default|GetBP_CharacterInventoryComponent)))
  (for _array_element _returnvalue
    (bind _value (Class|StructUtilsFunctionLibrary|GetInstancedStructValue _array_element)
      (:Valid
        (bind _value_2 (Class|StructUtilsFunctionLibrary|GetInstancedStructValue (.ItemDefinition (Utilities|Struct|BreakItemInstance _value)))
          (:Valid
            (if (== (.ItemType (Utilities|Struct|BreakItemDefinition _value_2)) "(TagName=\"Itemization.ItemType.Gold\")")
              (bind _outitemdrop (Class|ItemInventoryComponent|DropItem (Variables|Default|GetBP_CharacterInventoryComponent) (.ItemId (Utilities|Struct|BreakItemInstance _value))))
              (LocalVariables|SetLocalDroppedItem _outitemdrop)))))))
  (Utilities|IsValid (LocalVariables|GetLocalDroppedItem)
    (:Is%20Valid
      (CallFunction|SetItemDropLocation (LocalVariables|GetLocalDroppedItem))
      (CallFunction|ClientSucceededItemDrop (.ItemId (Utilities|Struct|BreakItemInstance _value))))
    (:Is%20Not%20Valid
      (CallFunction|ClientFailedItemDrop (.ItemId (Utilities|Struct|BreakItemInstance _value))))))

(fn ServerTryPickupItemImplementation
  (params (ItemDrop :type Item%20Drop%20Object%20Reference))
  (LocalVariables|SetLocalTryPickupItemInstance (Class|ItemDrop|GetItemInstance ItemDrop))
  ;[1 0 0] We push Gold straight into the Character Inventory.
  (if (== (.ItemType (Utilities|Struct|BreakItemDefinition (Class|ItemDrop|GetItemDefinitionStruct ItemDrop))) "(TagName=\"Itemization.ItemType.Gold\")")
    (bind (_itemid _returnvalue) (CallFunction|HasGold))
    (if _returnvalue
      (bind _returnvalue_2 (Class|ItemInventoryComponent|StackItemfromItemDrop (Variables|Default|GetBP_CharacterInventoryComponent) ItemDrop _itemid true))
      (if (not _returnvalue_2)
        (CallFunction|ClientFailedItemPickup)
        (else
          (CallFunction|ClientSucceededItemPickup (LocalVariables|GetLocalTryPickupItemInstance))))
      (else
        (bind _returnvalue_3 (Class|ItemInventoryComponent|TakeItemDrop :self (Variables|Default|GetBP_CharacterInventoryComponent) :ItemDrop ItemDrop))
        (if (not _returnvalue_3)
          (CallFunction|ClientFailedItemPickup)
          (else
            (CallFunction|ClientSucceededItemPickup (LocalVariables|GetLocalTryPickupItemInstance))))))
    (else
      (bind _returnvalue_4 (Class|ItemInventoryComponent|TakeItemDrop :self (Variables|Default|GetBP_CursorInventoryComponent) :ItemDrop ItemDrop))
      (if (not _returnvalue_4)
        (CallFunction|ClientFailedItemPickup)
        (else
          (CallFunction|ClientSucceededItemPickup (LocalVariables|GetLocalTryPickupItemInstance)))))))

(fn HasGold
  (bind _returnvalue (Class|ItemInventoryComponent|GetItems (Variables|Default|GetBP_CharacterInventoryComponent)))
  (for _array_element _returnvalue
    (bind _value (Class|StructUtilsFunctionLibrary|GetInstancedStructValue _array_element)
      (:Valid
        (bind _value_2 (Class|StructUtilsFunctionLibrary|GetInstancedStructValue (.ItemDefinition (Utilities|Struct|BreakItemInstance _value)))
          (:Valid
            (if (== (.ItemType (Utilities|Struct|BreakItemDefinition _value_2)) "(TagName=\"Itemization.ItemType.Gold\")")
              (LocalVariables|SetbLocalHasGold true)
              (LocalVariables|SetLocalGoldItemId (.ItemId (Utilities|Struct|BreakItemInstance _value)))))))))
  (return (LocalVariables|GetLocalGoldItemId) (LocalVariables|GetbLocalHasGold)))